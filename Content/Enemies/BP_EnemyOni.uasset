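; Oni enemy Blueprint with a close-range spin attack against the player.
; Box overlap starts an attack loop on a one-second delay while not stunned: a timeline spins yaw, then a debug-drawn sphere trace damages and launches the player along the Oni's forward vector.
; Incoming damage lowers Health, calls OnDeath at zero, and sets a burn timer for Fire damage.
; PlayerNearby is never cleared here, and the stun sequence is unconnected.
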(event OnComponentBeginOverlap(Box)
  (params (OverlappedComponent :type Primitive%20Component%20Object%20Reference) (OtherActor :type Actor%20Object%20Reference) (OtherComp :type Primitive%20Component%20Object%20Reference) (OtherBodyIndex :type Integer) (bFromSweep :type Boolean) (SweepResult :type Hit%20Result%20Structure%20%28by%20ref%29))
  (bind _returnvalue (Transformation|GetActorRotation))
  (bind _returnvalue_2 (Transformation|GetActorLocation))
  (bind _returnvalue_3 (Math|Vector|GetForwardVector _returnvalue))
  ;[1 1 1] Spin Attack
  ;;[1 1 1] Is that the Player
  (if (== OtherActor (Game|GetPlayerCharacter 0))
    (bind _output_get (Variables|Default|SetPlayer%20Nearby true))
    (if (Math|Boolean|ANDBoolean _output_get (Variables|Default|GetCanAttack) (not (Variables|Default|GetStunned))) :!label _label
      (Utilities|FlowControl|Sequence
        (:then_0
          ;;[1 1 1] Spin
          (bind _rotate (Timeline|Timeline PlayFromStart) ; Controls rotation alpha
            (:Update
              (Transformation|SetActorRotation (Math|Rotator|MakeRotator 0.0 0.0 (+ (.yaw (Transformation|GetActorRotation)) (* _rotate 3.6e+02)))))))
        (:then_1
          (Variables|Default|SetCanAttack false)
          ;;[1 1 1] Check If Player is still Nearby
          (Utilities|FlowControl|Delay 1.0)
          (bind _outhits (Collision|MultiSphereTraceForObjects _returnvalue_2 _returnvalue_2 2e+02 (Utilities|Array|MakeArray "ObjectTypeQuery3") false 0 "ForDuration" true "(R=1.000000,G=0.000000,B=0.000000,A=1.000000)" "(R=0.000000,G=1.000000,B=0.000000,A=1.000000)" 1.0))
          (for _array_element _outhits
            ;;[1 1 1] Damage Only Player
            (if (== (.hitactor _array_element) (Game|GetPlayerCharacter 0))
              (Game|Damage|ApplyDamage (.hitactor _array_element) 32.0 0 0)
              ;;[1 1 1] Launch Player
              (Character|LaunchCharacter (Game|GetPlayerCharacter 0) (Math|Vector|MakeVector (* (.x _returnvalue_3) 1.5e+03) (* (.y _returnvalue_3) 1.5e+03) 0.0) true true))))
        (:then_2
          (Utilities|FlowControl|Delay 1.0)
          (Variables|Default|SetCanAttack true)
          (goto _label))))))

(event Custom|CustomEvent
  ;[1 1 1] Spin Attack
  ;;[1 1 1] Spin
  (bind _rotate (Timeline|Timeline Stop) ; Controls rotation alpha
    (:Update
      (Transformation|SetActorRotation (Math|Rotator|MakeRotator 0.0 0.0 (+ (.yaw (Transformation|GetActorRotation)) (* _rotate 3.6e+02)))))))

(event EventBeginPlay
  (|CallParentFunction) ; This node is disabled and will not be called.\nDrag off pins to build functionality.
)

(event Collision|EventActorBeginOverlap
  (params (OtherActor :type Actor%20Object%20Reference)))

(event EventTick
  (params (DeltaSeconds :type Float%20%28single-precision%29))
  (|CallParentFunction DeltaSeconds) ; This node is disabled and will not be called.\nDrag off pins to build functionality.
)

(event Game|Damage|EventAnyDamage
  (params (Damage :type Float%20%28single-precision%29) (DamageType :type Damage%20Type%20Object%20Reference) (InstigatedBy :type Controller%20Object%20Reference) (DamageCauser :type Actor%20Object%20Reference))
  (bind _returnvalue (Utilities|GetDisplayName DamageType))
  (Development|PrintString _returnvalue)
  (if (Utilities|Enum|Equal(Enum) _returnvalue "Default__Fire_C")
    (bind _output_get (Variables|Default|SetTimeOnFire 1e+01))
    (Development|PrintString (Utilities|String|ToString(Float) _output_get)))
  (Variables|Default|SetHealth (- (Variables|Default|GetHealth) Damage))
  (if (<= (Variables|Default|GetHealth) 0.0)
    (CallFunction|OnDeath)))

(fn ConstructionScript
  (|CallParentFunction))