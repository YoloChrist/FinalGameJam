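; Base melee enemy Blueprint that chases the player, deals damage on contact, and drops loot when killed.
; Tick issues AIMoveTo at the player, and a Hit applies damage, then spins the actor via a timeline before a short cooldown re-enables attacking.
; Damage reduces health; below zero it ragdolls, then after a delay spawns random gold plus a chance-based item pickup and destroys itself.
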(event Custom|OnDeath
  ;[1 1 1] On Death.
  (Utilities|FlowControl|Sequence
    (:then_0
      ;;[1 1 1] Ragdoll
      (Components|Movement|StopMovementImmediately (Variables|Character|GetCharacterMovement))
      (Components|DestroyComponent (Variables|Collision|GetCapsuleComponent))
      (Physics|SetSimulatePhysics (Variables|Character|GetMesh) true))
    (:then_1
      (Utilities|FlowControl|Delay 0.8)
      (CallFunction|SpawnGold&Items))
    (:then_2
      (Utilities|FlowControl|Delay 0.8)
      (Actor|DestroyActor) ; Destory self
    )))

(event Collision|EventHit
  (params (MyComp :type Primitive%20Component%20Object%20Reference) (Other :type Actor%20Object%20Reference) (OtherComp :type Primitive%20Component%20Object%20Reference) (bSelfMoved :type Boolean) (HitLocation :type Vector :default "0, 0, 0") (HitNormal :type Vector :default "0, 0, 0") (NormalImpulse :type Vector :default "0, 0, 0") (Hit :type Hit%20Result%20Structure%20%28by%20ref%29))
  (bind _returnvalue (Game|GetPlayerCharacter 0))
  ;[1 1 1] On overlap with player, subtract health from player.
  (if (and (== Other _returnvalue) (Variables|Default|GetCanAttack))
    (Variables|Default|SetCanAttack false) ; Stop attacks whilst attacking
    (Game|Damage|ApplyDamage _returnvalue (Variables|Default|GetDamage) 0 0)
    ;[1 1 1] Rotate actor when attacking
    (bind _rotate (Timeline|Timeline PlayFromStart) ; Controls rotation alpha
      (:Update
        (Transformation|SetActorRotation (Math|Rotator|MakeRotator 0.0 0.0 (+ (.yaw (Transformation|GetActorRotation)) (* _rotate 3.6e+02)))))
      (:Finished
        (Utilities|FlowControl|Delay 0.5)
        (Variables|Default|SetCanAttack true) ; Allow next attack
      ))))

(event EventBeginPlay
  (bind _charactermovement (Variables|Character|GetCharacterMovement))
  ;[1 1 1] Set walk speed on spawn
  (Variables|/Script/Engine.CharacterMovementComponent|SetMaxWalkSpeed _charactermovement (* (Variables|/Script/Engine.CharacterMovementComponent|GetMaxWalkSpeed _charactermovement) (Variables|Default|GetSpeedMult))))

(event EventTick
  (params (DeltaSeconds :type Float%20%28single-precision%29))
  ;[1 1 1] Move to player
  (AI|AIMoveTo self "0, 0, 0" (Game|GetPlayerCharacter 0) 0.0 false))

(event Game|Damage|EventAnyDamage
  (params (Damage :type Float%20%28single-precision%29) (DamageType :type Damage%20Type%20Object%20Reference) (InstigatedBy :type Controller%20Object%20Reference) (DamageCauser :type Actor%20Object%20Reference))
  ;[1 1 1] When actor is hit, subtract health from damage. Then check if health is greater than 0.
  (Variables|Default|SetHealth (- (Variables|Default|GetHealth) Damage))
  (if (< (Variables|Default|GetHealth) 0.0)
    (CallFunction|OnDeath)))

(fn ConstructionScript)

(fn SpawnGold&Items
  (bind _returnvalue (Game|SpawnActorfromClass "/Game/Pickups/BP_GoldPickup.BP_GoldPickup_C" (Math|Transform|MakeTransform (Transformation|GetWorldLocation (Variables|Character|GetMesh)) "0, 0, 0" "1.000000,1.000000,1.000000") "Undefined" "MultiplyWithRoot" 0 0)) ; Spawn gold actor
  (Variables|/Game/Pickups/BP_GoldPickup.BP_GoldPickup_C|SetGold _returnvalue (Math|Random|RandomIntegerinRange 1 10))
  (if (< (Math|Random|RandomInteger 100) (Variables|Default|GetPickupChance)) ; Random chance to spawn pickup
    (Game|SpawnActorfromClass "/Game/Pickups/BP_ItemPickup.BP_ItemPickup_C" (Math|Transform|MakeTransform (Transformation|GetWorldLocation (Variables|Character|GetMesh)) "0, 0, 0" "1.000000,1.000000,1.000000") "Undefined" "MultiplyWithRoot" 0 0) ; Spawn the pickupable item actor
  ))