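; Master enemy that chases the player and performs a looping spin attack while nearby, dealing damage and knockback.
; A fast timer drives AIMoveTo, or launches the enemy away when stunned; stuns also cancel the spin.
; AnyDamage matches damage-type names to start burn or chance-based freeze, using Tick-driven DoOnce/Delay countdowns alongside the camera-facing health bar.
; Death ragdolls the body, drops gold and possible items, and heals the player via negative damage.
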(event OnComponentBeginOverlap(Box)
  (params (OverlappedComponent :type Primitive%20Component%20Object%20Reference) (OtherActor :type Actor%20Object%20Reference) (OtherComp :type Primitive%20Component%20Object%20Reference) (OtherBodyIndex :type Integer) (bFromSweep :type Boolean) (SweepResult :type Hit%20Result%20Structure%20%28by%20ref%29))
  (bind _returnvalue (Transformation|GetActorRotation))
  (bind _returnvalue_2 (Transformation|GetActorLocation))
  (bind _returnvalue_3 (Math|Vector|GetForwardVector _returnvalue))
  ;[1 1 1] Spin Attack
  ;;[1 1 1] Is that the Player
  (if (== OtherActor (Game|GetPlayerCharacter 0))
    (bind _output_get (Variables|Default|SetPlayer%20Nearby true))
    (if (Math|Boolean|ANDBoolean _output_get (Variables|Default|GetCanAttack) (not (Variables|Default|GetStunned))) :!label _label
      (Utilities|FlowControl|Sequence
        (:then_0
          ;;[1 1 1] Spin
          (bind _rotate (Timeline|Timeline_0 PlayFromStart) ; Controls rotation alpha
            (:Update
              (Transformation|SetActorRotation (Math|Rotator|MakeRotator 0.0 0.0 (+ (.yaw (Transformation|GetActorRotation)) (* _rotate 3.6e+02)))))))
        (:then_1
          (Variables|Default|SetCanAttack false)
          ;;[1 1 1] Check If Player is still Nearby
          (Utilities|FlowControl|Delay 0.5)
          (bind _outhits (Collision|MultiSphereTraceForObjects _returnvalue_2 _returnvalue_2 2e+02 (Utilities|Array|MakeArray "ObjectTypeQuery3") false 0 "None" true "(R=1.000000,G=0.000000,B=0.000000,A=1.000000)" "(R=0.000000,G=1.000000,B=0.000000,A=1.000000)" 1.0))
          (for _array_element _outhits
            ;;[1 1 1] Damage Only Player
            (if (== (.hitactor _array_element) (Game|GetPlayerCharacter 0))
              (Game|Damage|ApplyDamage (.hitactor _array_element) 2e+01 0 0)
              ;;[1 1 1] Launch Player
              (Character|LaunchCharacter (Game|GetPlayerCharacter 0) (Math|Vector|MakeVector (* (.x _returnvalue_3) 1.5e+03) (* (.y _returnvalue_3) 1.5e+03) 0.0) true true))))
        (:then_2
          (Utilities|FlowControl|Delay 1.0)
          (Variables|Default|SetCanAttack true)
          (goto _label))))))

(event OnComponentEndOverlap(Box)
  (params (OverlappedComponent :type Primitive%20Component%20Object%20Reference) (OtherActor :type Actor%20Object%20Reference) (OtherComp :type Primitive%20Component%20Object%20Reference) (OtherBodyIndex :type Integer))
  ;[1 1 1] Spin Attack
  (if (== OtherActor (Game|GetPlayerCharacter 0))
    (Variables|Default|SetPlayer%20Nearby false)))

(event Custom|OnAIMoveTo
  ;[1 1 1] Move to player
  (if (Variables|Default|GetStunned) ; Check if enemy is stunned
    ;[1 1 1] Launch Enemy
    (Utilities|FlowControl|DoOnce false :!label _label
      (:Completed
        (Class|NavMovementComponent|StopActiveMovement (Variables|Character|GetCharacterMovement)) ; Stop pathing
        (Character|LaunchCharacter (* (Math|Vector|Normalize (- (.location (Transformation|GetActorTransform)) (.location (Transformation|GetActorTransform (Game|GetPlayerCharacter 0)))) 1.0) "2000.000000,2000.000000,0.000000") false false)))
    (else
      (AI|AIMoveTo self "0, 0, 0" (Game|GetPlayerCharacter 0) 0.0 false
        (:then
          (goto _label Reset))))))

(event Custom|OnStunCancelAnim
  ;[1 1 1] Spin Attack
  ;;[1 1 1] Spin
  (bind _rotate (Timeline|Timeline_0 Stop) ; Controls rotation alpha
    (:Update
      (Transformation|SetActorRotation (Math|Rotator|MakeRotator 0.0 0.0 (+ (.yaw (Transformation|GetActorRotation)) (* _rotate 3.6e+02)))))))

(event Custom|OnDeath
  ;[1 1 1] On Death.
  (Utilities|FlowControl|Sequence
    (:then_0
      ;;[1 1 1] Ragdoll
      (Components|Movement|StopMovementImmediately (Variables|Character|GetCharacterMovement))
      (Components|DestroyComponent (Variables|Collision|GetCapsuleComponent))
      (Physics|SetSimulatePhysics (Variables|Character|GetMesh) true)
      (Utilities|FlowControl|DelayUntilNextTick)
      (Physics|AddImpulse (Variables|Character|GetMesh) (* (Math|Vector|Normalize (- (.location (Transformation|GetActorTransform)) (.location (Transformation|GetActorTransform (Game|GetPlayerCharacter 0))))) "-5000.000000,-5000.000000,0.000000") "None" false))
    (:then_1
      (Utilities|FlowControl|Delay 0.8)
      (CallFunction|SpawnGold&Items)
      (Game|Damage|ApplyDamage (Game|GetPlayerCharacter 0) -2e+01 0 0))
    (:then_2
      (Utilities|FlowControl|Delay 0.8)
      (Actor|DestroyActor) ; Destory self
    )))

(event EventTick
  (params (DeltaSeconds :type Float%20%28single-precision%29))
  (bind _health_bar_widget (Variables|Default|GetHealth%20Bar%20Widget))
  ;[1 1 1] Health bar
  (bind _aswb_health_bar (Utilities|Casting|CastToWB_HealthBar (UserInterface|GetWidget (Variables|Default|GetHealth%20Bar%20Widget)))
    (:then
      (Progress|SetPercent (Variables|/Game/Enemies/WB_HealthBar.WB_HealthBar_C|GetHealthBar _aswb_health_bar) (/ (Variables|Default|GetHealth) (Variables|Default|GetStartHealth)))
      (Transformation|SetWorldRotation _health_bar_widget (Math|Rotator|FindLookatRotation (Transformation|GetWorldLocation _health_bar_widget) (Transformation|GetWorldLocation (Variables|/Script/Engine.PlayerCameraManager|GetTransformComponent (Game|GetPlayerCameraManager 0)))) false false))
    (:CastFailed
      _))
  ;[1 1 1] Fire damage
  (Utilities|FlowControl|Sequence
    (:then_0
      (if (> (Variables|Default|GetTimeOnFire) 0.0)
        (Utilities|FlowControl|DoOnce false :!label _label
          (:Completed
            (Variables|Default|SetHealth (- (Variables|Default|GetHealth) 2e+01))
            (Variables|Default|SetTimeOnFire (- (Variables|Default|GetTimeOnFire) 1.0))
            (if (<= (Variables|Default|GetHealth) 0.0)
              (CallFunction|OnDeath)
              (else
                (Utilities|FlowControl|Delay 1.0)
                (goto _label Reset)))))))
    (:then_1
      ;[1 1 1] Freeze effect
      (if (> (Variables|Default|GetTimeFrozen) 0.0)
        (Utilities|FlowControl|DoOnce false :!label _label_2
          (:Completed
            (Variables|Default|SetTimeFrozen (- (Variables|Default|GetTimeFrozen) 0.1))
            (Variables|Default|SetStunned true)
            (CallFunction|OnStunCancelAnim)
            (Utilities|FlowControl|Delay 0.1)
            (if (> (Variables|Default|GetTimeFrozen) 0.0)
              (goto _label_2 Reset)
              (else
                (Variables|Default|SetStunned false)
                (goto _label_2 Reset)))))))))

(event EventBeginPlay
  ;[1 1 1] Set walk speed on spawn
  (Variables|Default|SetStartHealth (Variables|Default|GetHealth))
  (|SetWalkSpeedOnSpawn)
  (Utilities|Time|SetTimerbyEvent (delegate Custom|OnAIMoveTo) 0.01 true true))

(event Game|Damage|EventAnyDamage
  (params (Damage :type Float%20%28single-precision%29) (DamageType :type Damage%20Type%20Object%20Reference) (InstigatedBy :type Controller%20Object%20Reference) (DamageCauser :type Actor%20Object%20Reference))
  (bind _returnvalue (Utilities|GetDisplayName DamageType))
  ;[1 1 1] When actor is hit, subtract health from damage. Then check if health is greater than 0.
  (if (Utilities|Enum|Equal(Enum) _returnvalue "Default__Fire_C")
    (Variables|Default|SetTimeOnFire 1e+01)
    (elif (Utilities|Enum|Equal(Enum) _returnvalue "Default__Ice_C")
      (if (== (Math|Random|RandomIntegerinRange 0 2) 0)
        (Variables|Default|SetTimeFrozen 3.0))))
  (Variables|Default|SetHealth (- (Variables|Default|GetHealth) Damage))
  (if (<= (Variables|Default|GetHealth) 0.0)
    (CallFunction|OnDeath)
    (elif (not (> (Variables|Default|GetTimeFrozen) 0.0))
      (Utilities|FlowControl|Sequence
        (:then_0
          (Variables|Default|SetStunned true)
          (CallFunction|OnStunCancelAnim))
        (:then_1
          (Utilities|FlowControl|Delay 1.0)
          (Variables|Default|SetStunned false))))))

(fn ConstructionScript)

(fn SpawnGold&Items
  (Utilities|FlowControl|Sequence
    (:then_0
      (bind _returnvalue (Game|SpawnActorfromClass "/Game/Pickups/BP_GoldPickup.BP_GoldPickup_C" (Math|Transform|MakeTransform (Transformation|GetWorldLocation (Variables|Default|GetSpawn%20Location)) "0, 0, 0" "1.000000,1.000000,1.000000") "Undefined" "MultiplyWithRoot" 0 0)) ; Spawn gold actor
      (Variables|/Game/Pickups/BP_GoldPickup.BP_GoldPickup_C|SetGold _returnvalue (Math|Random|RandomIntegerinRange 1 10)))
    (:then_1
      (if (< (Math|Random|RandomInteger 100) (Variables|Default|GetPickupChance)) ; Random chance to spawn pickup
        (Game|SpawnActorfromClass "/Game/Pickups/BP_ItemPickup.BP_ItemPickup_C" (Math|Transform|MakeTransform (Transformation|GetWorldLocation (Variables|Default|GetSpawn%20Location)) "0, 0, 0" "1.000000,1.000000,1.000000") "Undefined" "MultiplyWithRoot" 0 0) ; Spawn the pickupable item actor
      ))))

(fn AttackPlayer
  (bind _returnvalue (Transformation|GetActorLocation))
  (bind _outhits (Collision|MultiSphereTraceForObjects _returnvalue _returnvalue 2e+02 (Utilities|Array|MakeArray "ObjectTypeQuery3") false 0 "ForDuration" true "(R=1.000000,G=0.000000,B=0.000000,A=1.000000)" "(R=0.000000,G=1.000000,B=0.000000,A=1.000000)" 1.0))
  (for _array_element _outhits
    (if (== (.hitactor _array_element) (Game|GetPlayerCharacter 0))
      (Game|Damage|ApplyDamage (.hitactor _array_element) 2e+01 0 0))))