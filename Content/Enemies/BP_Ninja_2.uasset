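; Ranged ninja enemy that chases the player, holds position inside a set range and fires projectiles.
; A fast looping timer either paths toward the player, halts, or, when stunned, launches the ninja horizontally away once, with the launch re-armed when chasing resumes.
; Tick turns it toward the player and spawns projectiles from ShootHere, throttled by DoOnce and Delay, regardless of stun or distance.
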(event Custom|CustomEvent
  (if (Variables|Default|GetStunned) ; Check if enemy is stunned
    ;[1 1 1] Launch Enemy
    (Utilities|FlowControl|DoOnce false :!label _label
      (:Completed
        (Class|NavMovementComponent|StopActiveMovement (Variables|Character|GetCharacterMovement)) ; Stop pathing
        (Character|LaunchCharacter (* (Math|Vector|Normalize (- (.location (Transformation|GetActorTransform)) (.location (Transformation|GetActorTransform (Game|GetPlayerCharacter 0)))) 1.0) "2000.000000,2000.000000,0.000000") false false)))
    (elif (>= (Math|Vector|Distance(Vector) (Transformation|GetActorLocation) (Transformation|GetActorLocation (Game|GetPlayerCharacter 0))) 6e+02)
      (AI|AIMoveTo self "0, 0, 0" (Game|GetPlayerCharacter 0) 0.0 false
        (:then
          (goto _label Reset)))
      (else
        (Components|Movement|StopMovementImmediately (Variables|Character|GetCharacterMovement))))))

(event EventTick
  (params (DeltaSeconds :type Float%20%28single-precision%29))
  (Utilities|FlowControl|Sequence
    (:then_0
      (Transformation|SetActorRotation (Math|Rotator|FindRelativeLookatRotation (Math|Conversions|ToTransform(Vector) (Transformation|GetActorLocation)) (Transformation|GetActorLocation (Game|GetPlayerCharacter 0)))))
    (:then_1
      (Utilities|FlowControl|DoOnce false :!label _label
        (:Completed
          (Game|SpawnActorfromClass "/Game/Enemies/BP_Enemy_Projectile.BP_Enemy_Projectile_C" (Transformation|GetWorldTransform (Variables|Default|GetShootHere)) "AlwaysSpawn" "MultiplyWithRoot" 0 0)
          (Utilities|FlowControl|Delay 1.0)
          (goto _label Reset))))))

(event EventBeginPlay
  (bind _charactermovement (Variables|Character|GetCharacterMovement))
  ;[1 1 1] Set walk speed on spawn
  (Variables|/Script/Engine.CharacterMovementComponent|SetMaxWalkSpeed _charactermovement (* (Variables|/Script/Engine.CharacterMovementComponent|GetMaxWalkSpeed _charactermovement) (Variables|Default|GetSpeedMult)))
  (Utilities|Time|SetTimerbyEvent (delegate Custom|CustomEvent) 0.01 true true))

(fn ConstructionScript
  (|CallParentFunction))