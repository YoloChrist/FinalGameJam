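; Ranged enemy that chases the player, always faces them and fires a projectile every second.
; A looping timer drives pathing, halting within 600 units, or launches the enemy away once when stunned.
; Damage stuns it for a second; death ragdolls it with an impulse, spawns random gold and a chance item, then destroys it.
; AttackPlayer defines a sphere-trace melee hit but is not called here.
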(event Custom|OnAIMoveTo
  (if (Variables|Default|GetStunned) ; Check if enemy is stunned
    ;[1 1 1] Launch Enemy
    (Utilities|FlowControl|DoOnce false :!label _label
      (:Completed
        (Class|NavMovementComponent|StopActiveMovement (Variables|Character|GetCharacterMovement)) ; Stop pathing
        (Character|LaunchCharacter (* (Math|Vector|Normalize (- (.location (Transformation|GetActorTransform)) (.location (Transformation|GetActorTransform (Game|GetPlayerCharacter 0)))) 1.0) "2000.000000,2000.000000,0.000000") false false)))
    (elif (>= (Math|Vector|Distance(Vector) (Transformation|GetActorLocation) (Transformation|GetActorLocation (Game|GetPlayerCharacter 0))) 6e+02)
      (AI|AIMoveTo self "0, 0, 0" (Game|GetPlayerCharacter 0) 0.0 false
        (:then
          (goto _label Reset)))
      (else
        (Components|Movement|StopMovementImmediately (Variables|Character|GetCharacterMovement))))))

(event Custom|OnDeath
  ;[1 1 1] On Death.
  (Utilities|FlowControl|Sequence
    (:then_0
      ;;[1 1 1] Ragdoll
      (Components|Movement|StopMovementImmediately (Variables|Character|GetCharacterMovement))
      (Components|DestroyComponent (Variables|Collision|GetCapsuleComponent))
      (Physics|SetSimulatePhysics (Variables|Character|GetMesh) true)
      (Utilities|FlowControl|DelayUntilNextTick)
      (Physics|AddImpulse (Variables|Character|GetMesh) (* (Math|Vector|Normalize (- (.location (Transformation|GetActorTransform)) (.location (Transformation|GetActorTransform (Game|GetPlayerCharacter 0))))) "-5000.000000,-5000.000000,0.000000") "None" false))
    (:then_1
      (Utilities|FlowControl|Delay 0.8)
      (CallFunction|SpawnGold&Items))
    (:then_2
      (Utilities|FlowControl|Delay 0.8)
      (Actor|DestroyActor) ; Destory self
    )))

(event EventTick
  (params (DeltaSeconds :type Float%20%28single-precision%29))
  (Utilities|FlowControl|Sequence
    (:then_0
      (Transformation|SetActorRotation (Math|Rotator|FindRelativeLookatRotation (Math|Conversions|ToTransform(Vector) (Transformation|GetActorLocation)) (Transformation|GetActorLocation (Game|GetPlayerCharacter 0)))))
    (:then_1
      (Utilities|FlowControl|DoOnce false :!label _label
        (:Completed
          (Game|SpawnActorfromClass "/Game/Enemies/BP_Enemy_Projectile.BP_Enemy_Projectile_C" (Transformation|GetWorldTransform (Variables|Default|GetShooting_here)) "AlwaysSpawn" "MultiplyWithRoot" 0 0)
          (Utilities|FlowControl|Delay 1.0)
          (goto _label Reset))))))

(event EventBeginPlay
  (bind _charactermovement (Variables|Character|GetCharacterMovement))
  ;[1 1 1] Set walk speed on spawn
  (Variables|/Script/Engine.CharacterMovementComponent|SetMaxWalkSpeed _charactermovement (* (Variables|/Script/Engine.CharacterMovementComponent|GetMaxWalkSpeed _charactermovement) (Variables|Default|GetSpeedMult)))
  (Utilities|Time|SetTimerbyEvent (delegate Custom|OnAIMoveTo) 0.01 true true))

(event Game|Damage|EventAnyDamage
  (params (Damage :type Float%20%28single-precision%29) (DamageType :type Damage%20Type%20Object%20Reference) (InstigatedBy :type Controller%20Object%20Reference) (DamageCauser :type Actor%20Object%20Reference))
  ;[1 1 1] When actor is hit, subtract health from damage. Then check if health is greater than 0.
  (Variables|Default|SetHealth (- (Variables|Default|GetHealth) Damage))
  (if (< (Variables|Default|GetHealth) 0.0)
    (CallFunction|OnDeath)
    (else
      (Utilities|FlowControl|Sequence
        (:then_0
          (Variables|Default|SetStunned true))
        (:then_1
          (Utilities|FlowControl|Delay 1.0)
          (Variables|Default|SetStunned false))))))

(fn ConstructionScript)

(fn SpawnGold&Items
  (Utilities|FlowControl|Sequence
    (:then_0
      (bind _returnvalue (Game|SpawnActorfromClass "/Game/Pickups/BP_GoldPickup.BP_GoldPickup_C" (Math|Transform|MakeTransform (Transformation|GetWorldLocation (Variables|Character|GetMesh)) "0, 0, 0" "1.000000,1.000000,1.000000") "Undefined" "MultiplyWithRoot" 0 0)) ; Spawn gold actor
      (Variables|/Game/Pickups/BP_GoldPickup.BP_GoldPickup_C|SetGold _returnvalue (Math|Random|RandomIntegerinRange 1 10)))
    (:then_1
      (if (< (Math|Random|RandomInteger 100) (Variables|Default|GetPickupChance)) ; Random chance to spawn pickup
        (Game|SpawnActorfromClass "/Game/Pickups/BP_ItemPickup.BP_ItemPickup_C" (Math|Transform|MakeTransform (Transformation|GetWorldLocation (Variables|Character|GetMesh)) "0, 0, 0" "1.000000,1.000000,1.000000") "Undefined" "MultiplyWithRoot" 0 0) ; Spawn the pickupable item actor
      ))))

(fn AttackPlayer
  (bind _returnvalue (Transformation|GetActorLocation))
  (bind _outhits (Collision|MultiSphereTraceForObjects _returnvalue _returnvalue 2e+02 (Utilities|Array|MakeArray "ObjectTypeQuery3") false 0 "ForDuration" true "(R=1.000000,G=0.000000,B=0.000000,A=1.000000)" "(R=0.000000,G=1.000000,B=0.000000,A=1.000000)" 1.0))
  (for _array_element _outhits
    (if (== (.hitactor _array_element) (Game|GetPlayerCharacter 0))
      (Game|Damage|ApplyDamage (.hitactor _array_element) 2e+01 0 0))))