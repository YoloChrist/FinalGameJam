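; Gold pickup Blueprint that adds a random amount of gold to the player's total when collected.
; On BeginPlay it rolls its gold value within a small fixed range.
; Its Pickup override adds that value to the Gold stored in BP_GameInstance and destroys the actor before calling the parent Pickup.
; If the game instance cast fails, the override stops without destroying the actor or calling the parent.
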(event EventBeginPlay
  (Variables|Default|SetGold (Math|Random|RandomIntegerinRange 1 10)))

(fn ConstructionScript
  (|CallParentFunction))

(fn Pickup
  (params (Ref_BP_ThirdPersonCharacter :type BP%20Third%20Person%20Character%20Object%20Reference))
  (bind _asbp_game_instance (Utilities|Casting|CastToBP_GameInstance (Game|GetGameInstance)))
  (Variables|/Game/Blueprints/BP_GameInstance.BP_GameInstance_C|SetGold _asbp_game_instance (+ (Variables|Default|GetGold) (Variables|/Game/Blueprints/BP_GameInstance.BP_GameInstance_C|GetGold _asbp_game_instance)))
  (Actor|DestroyActor)
  (|CallParentFunction 0))