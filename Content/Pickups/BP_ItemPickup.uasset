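; Item pickup that offers the player a random unlocked item through a pickup widget.
; On BeginPlay it picks from the GameInstance's unlocked items and stores that item's data in ItemID.
; Its Pickup override opens UI_PickupItem only if none is showing, passes it the item, itself and the character's inventory component, then calls the parent.
; The widget is removed when the player stops overlapping.
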(event Collision|EventActorEndOverlap
  (params (OtherActor :type Actor%20Object%20Reference))
  (if (== OtherActor (Game|GetPlayerCharacter 0))
    (Class|GameViewportSubsystem|RemoveWidget (|GameViewportSubsystem) (Variables|Default|GetRef_UI))))

(event EventBeginPlay
  (bind _asbp_game_instance (Utilities|Casting|CastToBP_GameInstance (Game|GetGameInstance)))
  (bind _out_row (Default|GetUnlockedItemData _asbp_game_instance (.OutItem (Utilities|Array|Random (Variables|/Game/Blueprints/BP_GameInstance.BP_GameInstance_C|GetGetUnlockedItems _asbp_game_instance))))) ; Get random unlocked item
  (Variables|Default|SetItemID _out_row))

(fn ConstructionScript
  (|CallParentFunction))

(fn Pickup
  (params (Ref_BP_ThirdPersonCharacter :type BP%20Third%20Person%20Character%20Object%20Reference))
  (bind _foundwidgets (Widget|GetAllWidgetsOfClass "/Game/UI/UI_PickupItem.UI_PickupItem_C" true))
  (if (Utilities|Array|IsEmpty _foundwidgets)
    (bind _returnvalue (UserInterface|CreateWidget "/Game/UI/UI_PickupItem.UI_PickupItem_C" (Game|GetPlayerController 0)))
    (bind _output_get (Variables|Default|SetRef_UI _returnvalue))
    (UserInterface|Viewport|AddtoViewport _returnvalue 0)
    (Default|OnPickupOverlap _returnvalue (Variables|Default|GetItemID) self (Variables|/Game/ThirdPerson/Blueprints/BP_ThirdPersonCharacter.BP_ThirdPersonCharacter_C|GetBP_InventoryComponent Ref_BP_ThirdPersonCharacter))
    (|CallParentFunction 0)))