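; BP_MasterRoom is a procedural dungeon room that starts its enemy spawners when the player enters.
; On BeginPlay it binds to the dungeon generator's DungeonGenerationComplete dispatcher, which sets CanSpawn.
; Player overlap with RoomOverlapBox1 while CanSpawn is true calls StartSpawner on the room's BP_MasterEnemySpawner child actors.
; No guard prevents repeat calls on re-entry.
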(event OnComponentBeginOverlap(RoomOverlapBox1)
  (params (OverlappedComponent :type Primitive%20Component%20Object%20Reference) (OtherActor :type Actor%20Object%20Reference) (OtherComp :type Primitive%20Component%20Object%20Reference) (OtherBodyIndex :type Integer) (bFromSweep :type Boolean) (SweepResult :type Hit%20Result%20Structure%20%28by%20ref%29))
  ;[1 1 1] Check if player is in room and dungeon generation is complete.
  (if (and (== OtherActor (Game|GetPlayerCharacter 0)) (Variables|Default|GetCanSpawn))
    (CallFunction|OnPlayerEnter)))

(event Custom|OnPlayerEnter
  ;[1 1 1] Start spawning for all spawners in the room
  (for _array_element (Actor|GetAllChildActors false)
    (bind _asbp_master_enemy_spawner (Utilities|Casting|CastToBP_MasterEnemySpawner _array_element))
    (Default|StartSpawner _asbp_master_enemy_spawner)))

(event Custom|SetCanSpawn
  ;[1 1 1] Bind SetCanSpawn to DungeonGenerationComplete dispatcher in BP_DungeonGenerator
  (Variables|Default|SetCanSpawn true))

(event EventBeginPlay
  ;[1 1 1] Bind SetCanSpawn to DungeonGenerationComplete dispatcher in BP_DungeonGenerator
  (bind _returnvalue (Actor|GetActorOfClass "/Game/ProceduralDungeon/BP_DungeonGenerator.BP_DungeonGenerator_C"))
  (EventDispatchers|BindEventtoDungeonGenerationComplete _returnvalue (delegate Custom|SetCanSpawn)))

(fn ConstructionScript)